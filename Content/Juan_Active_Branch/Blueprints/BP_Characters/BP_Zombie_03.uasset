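; BP_Zombie_03 is a zombie enemy that chases the player, attacks in melee and takes damage.
; AIMoveTo targets the player controller, retrying on failure and attacking on success, while PawnSensing switches walk speed to a random run speed.
; Random montages drive attacks and hit reactions, with an attack notify applying sphere-overlap damage.
; Zero health calls Death, but that event is empty; its montage, kill report and destroy logic sit disconnected.
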(event OnSeePawn(PawnSensing)
  (params (Pawn :type Pawn%20Object%20Reference))
  (bind _runspeedarray (Variables|Default|GetRunSpeedArray))
  ;[1 1 1] Increase zombie speed when target spotted
  (Variables|/Script/Engine.CharacterMovementComponent|SetMaxWalkSpeed (Variables|Character|GetCharacterMovement) (Utilities|Array|Get(acopy) _runspeedarray (Math|Random|RandomInteger (Utilities|Array|Length _runspeedarray)))))

(event Custom|ChasePlayer
  ;[1 1 1] Follow main character
  (if (not (Variables|Default|GetisDead))
    (AI|AIMoveTo self "0, 0, 0" (Game|GetPlayerController 0) 4e+01 false
      (:OnSuccess
        (CallFunction|Attack))
      (:OnFail
        (CallFunction|ChasePlayer)))))

(event Custom|Attack
  (bind _attackarray (Variables|Default|GetAttackArray))
  ;[1 1 1] Attack + randomize anim
  (Animation|Montage|PlayMontage (Variables|Character|GetMesh) (Utilities|Array|Get(acopy) _attackarray (Math|Random|RandomInteger (Utilities|Array|Length _attackarray)))
    (:OnCompleted
      (CallFunction|ChasePlayer))
    (:OnNotifyBegin
      (Audio|PlaySoundatLocation "/Game/Juan_Active_Branch/SFX/Attack_cue.Attack_cue" (Transformation|GetActorLocation) "0, 0, 0" 1.0 1.0 0.0 0 0 0 0)
      (bind (_outactors _returnvalue) (Collision|SphereOverlapActors (Transformation|GetWorldLocation (Variables|Default|GetArrow1)) 8e+01 (Utilities|Array|MakeArray "ObjectTypeQuery3") 0 (Utilities|Array|MakeArray self)))
      (if _returnvalue
        (for _array_element _outactors
          (Game|Damage|ApplyDamage _array_element 2e+01 (Pawn|GetController) self "/Script/Engine.DamageType"))))))

(event Custom|Death
  ;[1 1 1] Death zombie
)

(event EventBeginPlay
  (bind _walkspeedarray (Variables|Default|GetWalkSpeedArray))
  ;[1 1 1] Call chase player
  (Utilities|FlowControl|Sequence
    (:then_0
      (CallFunction|ChasePlayer))
    (:then_1
      (Variables|Default|SetHealth (Variables|Default|GetMax%20Health)))
    (:then_2
      (Variables|/Script/Engine.CharacterMovementComponent|SetMaxWalkSpeed (Variables|Character|GetCharacterMovement) (Utilities|Array|Get(acopy) _walkspeedarray (Math|Random|RandomInteger (Utilities|Array|Length _walkspeedarray)))))))

(event Game|Damage|EventAnyDamage
  (params (Damage :type Float%20%28single-precision%29) (DamageType :type Damage%20Type%20Object%20Reference) (InstigatedBy :type Controller%20Object%20Reference) (DamageCauser :type Actor%20Object%20Reference))
  (bind _hitarray (Variables|Default|GethitArray))
  ;[1 1 1] Damage zombie
  (if (not (Variables|Default|GetisDead))
    (Development|PrintString "HIT!")
    (if (<= (Variables|Default|GetHealth) 0.0)
      (CallFunction|Death)
      (else
        (bind _output_get (Variables|Default|SetHealth (Math|Float|Clamp(Float) (- (Variables|Default|GetHealth) Damage) 0.0 (Variables|Default|GetMax%20Health))))
        (Development|PrintString (Utilities|String|ToString(Float) _output_get))
        (if (<= _output_get 0.0)
          (CallFunction|Death)
          (else
            (Animation|Montage|PlayMontage (Variables|Character|GetMesh) (Utilities|Array|Get(acopy) _hitarray (Math|Random|RandomInteger (Utilities|Array|Length _hitarray))))))))))

(fn ConstructionScript)