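; Main game mode that manages a pausing skill selection menu.
; On BeginPlay it creates and initializes a collapsed WB_SkillsUI widget, which ActivateSkillUI shows while pausing the game and switching to cursor and UI-only input.
; The Nitro, Flame Thrower and Mines events hide the menu and restore gameplay, but only print debug text in place of skill logic.
; Two generic skill events are print-only placeholders.
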(event EventActivateNitro
  (bind _returnvalue (Game|GetPlayerController 0))
  (Development|PrintString "ACTIVATE Nitro")
  (Variables|/Script/UMG.Widget|SetVisibility (Variables|Default|GetSkillsUI) "Collapsed")
  (Variables|/Script/Engine.PlayerController|SetbShowMouseCursor _returnvalue false)
  (Game|SetGamePaused false)
  (Input|SetInputModeGameOnly _returnvalue false))

(event EventActivateFlameThrower
  (bind _returnvalue (Game|GetPlayerController 0))
  (Development|PrintString "ACTIVATE Flame")
  (Variables|/Script/UMG.Widget|SetVisibility (Variables|Default|GetSkillsUI) "Collapsed")
  (Variables|/Script/Engine.PlayerController|SetbShowMouseCursor _returnvalue false)
  (Game|SetGamePaused false)
  (Input|SetInputModeGameOnly _returnvalue false))

(event EventBeginPlay
  (|CallParentFunction)
  ;[1 1 1] Create Skills Widget
  (bind _returnvalue (UserInterface|CreateWidget "/Game/Kirill_Active_Branch/WB_SkillsUI.WB_SkillsUI_C"))
  (bind _output_get (Variables|Default|SetSkillsUI _returnvalue))
  (UserInterface|Viewport|AddtoViewport _output_get 100)
  (Variables|/Script/UMG.Widget|SetVisibility (Variables|Default|GetSkillsUI) "Collapsed")
  (Class|SkillsWidget|InitWidget (Variables|Default|GetSkillsUI))
  (Variables|/Script/UMG.UserWidget|SetbIsFocusable (Variables|Default|GetSkillsUI) true))

(event EventActivateMines
  (bind _returnvalue (Game|GetPlayerController 0))
  (Development|PrintString "ACTIVATE Mines")
  (Variables|/Script/UMG.Widget|SetVisibility (Variables|Default|GetSkillsUI) "Collapsed")
  (Variables|/Script/Engine.PlayerController|SetbShowMouseCursor _returnvalue false)
  (Game|SetGamePaused false)
  (Input|SetInputModeGameOnly _returnvalue false))

(event EventActivateSkillUI
  (bind _returnvalue (Game|GetPlayerController 0))
  ;[1 1 1] Display Skill UI
  (Variables|/Script/UMG.Widget|SetVisibility (Variables|Default|GetSkillsUI) "Visible")
  (Game|SetGamePaused true)
  (Variables|/Script/Engine.PlayerController|SetbShowMouseCursor _returnvalue true)
  (Input|SetInputModeUIOnly _returnvalue (Variables|Default|GetSkillsUI) "DoNotLock" false))

(event EventGenericSkillTemp2
  (Development|PrintString "gen2"))

(event EventGenericSkillTemp1
  (Development|PrintString "gen1"))

(fn ConstructionScript)